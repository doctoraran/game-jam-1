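; BP_Enemy is an enemy actor configured from a Type asset that supplies its sprite and max health.
; On BeginPlay it applies that sprite and health, then registers itself with the GameState through a turn message.
; Its Attack event reports a 1-damage attack to the GameState, naming itself as the attacker.
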(event EventBeginPlay
  (bind _type (Variables|Default|GetType))
  (bind (_type_2 _maxhealth _sprite) (Utilities|Struct|BreakS_EnemyType _type))
  (Rendering|Components|Sprite|SetSprite (Variables|Default|GetSprite) _sprite)
  (Variables|Default|SetHealth _maxhealth)
  (Class|BPIRegisterTurn|RegisterTurn(Message) (Game|GetGameState) self))

(event EventAttack
  (Class|BPIAttack|Attack(Message) (Game|GetGameState) 1 self))

(fn ConstructionScript)