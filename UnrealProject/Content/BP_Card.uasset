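; BP_Card is a water and ice themed card for a card game, with one Blueprint covering every card type.
; The Construction Script switches on CardType to set the Paper2D sprite and the attack, defense, status effect, status value and energy cost.
; All card data is hard-coded in that switch, and the Event Graph is empty, so the card only holds data and visuals.
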(event EventBeginPlay)

(event Collision|EventActorBeginOverlap
  (params (OtherActor :type Actor%20Object%20Reference)))

(event EventTick
  (params (DeltaSeconds :type Float%20%28single-precision%29)))

(fn ConstructionScript
  (switch Utilities|FlowControl|Switch|SwitchonE_CardType (Variables|Default|GetCardType)
    (:NewEnumerator0
      (Rendering|Components|Sprite|SetSprite (Variables|Default|GetPaperSprite) "/Game/Assets/Cards/bubble_card_Sprite.bubble_card_Sprite")
      (Variables|Default|SetAttack 0)
      (Variables|Default|SetDefense 0)
      (Variables|Default|SetStatusEffect "NewEnumerator3")
      (Variables|Default|SetStatusValue 10)
      (Variables|Default|SetEnergyCost 2))
    (:NewEnumerator1
      (Rendering|Components|Sprite|SetSprite (Variables|Default|GetPaperSprite) "/Game/Assets/Cards/flood_card_Sprite.flood_card_Sprite")
      (Variables|Default|SetAttack 0)
      (Variables|Default|SetDefense 0)
      (Variables|Default|SetStatusEffect "NewEnumerator1")
      (Variables|Default|SetStatusValue 10)
      (Variables|Default|SetEnergyCost 2))
    (:NewEnumerator2
      (Rendering|Components|Sprite|SetSprite (Variables|Default|GetPaperSprite) "/Game/Assets/Cards/Freeze_card_Sprite.Freeze_card_Sprite")
      (Variables|Default|SetAttack 0)
      (Variables|Default|SetDefense 0)
      (Variables|Default|SetStatusEffect "NewEnumerator0")
      (Variables|Default|SetStatusValue 2)
      (Variables|Default|SetEnergyCost 2))
    (:NewEnumerator3
      (Rendering|Components|Sprite|SetSprite (Variables|Default|GetPaperSprite) "/Game/Assets/Cards/Ice_Shield_card_Sprite.Ice_Shield_card_Sprite")
      (Variables|Default|SetAttack 0)
      (Variables|Default|SetDefense 5)
      (Variables|Default|SetStatusEffect "NewEnumerator4")
      (Variables|Default|SetStatusValue 0)
      (Variables|Default|SetEnergyCost 1))
    (:NewEnumerator4
      (Rendering|Components|Sprite|SetSprite (Variables|Default|GetPaperSprite) "/Game/Assets/Cards/Ice_wall_card_Sprite.Ice_wall_card_Sprite")
      (Variables|Default|SetAttack 0)
      (Variables|Default|SetDefense 20)
      (Variables|Default|SetStatusEffect "NewEnumerator4")
      (Variables|Default|SetStatusValue 0)
      (Variables|Default|SetEnergyCost 3))
    (:NewEnumerator5
      (Rendering|Components|Sprite|SetSprite (Variables|Default|GetPaperSprite) "/Game/Assets/Cards/Splash_Card_Sprite.Splash_Card_Sprite")
      (Variables|Default|SetAttack 5)
      (Variables|Default|SetDefense 0)
      (Variables|Default|SetStatusEffect "NewEnumerator4")
      (Variables|Default|SetStatusValue 0)
      (Variables|Default|SetEnergyCost 1))
    (:NewEnumerator6
      (Rendering|Components|Sprite|SetSprite (Variables|Default|GetPaperSprite) "/Game/Assets/Cards/tsunami_card_Sprite.tsunami_card_Sprite")
      (Variables|Default|SetAttack 5)
      (Variables|Default|SetDefense 0)
      (Variables|Default|SetStatusEffect "NewEnumerator4")
      (Variables|Default|SetStatusValue 0)
      (Variables|Default|SetEnergyCost 3))
    (:NewEnumerator8
      (Rendering|Components|Sprite|SetSprite (Variables|Default|GetPaperSprite) "/Game/Assets/Cards/undercurrent_card_Sprite.undercurrent_card_Sprite")
      (Variables|Default|SetAttack 20)
      (Variables|Default|SetDefense 0)
      (Variables|Default|SetStatusEffect "NewEnumerator4")
      (Variables|Default|SetStatusValue 0)
      (Variables|Default|SetEnergyCost 1))
    (:NewEnumerator7
      (Rendering|Components|Sprite|SetSprite (Variables|Default|GetPaperSprite) "/Game/Assets/Cards/wave_card_Sprite.wave_card_Sprite")
      (Variables|Default|SetAttack 5)
      (Variables|Default|SetDefense 0)
      (Variables|Default|SetStatusEffect "NewEnumerator1")
      (Variables|Default|SetStatusValue 5)
      (Variables|Default|SetEnergyCost 2))
    (:NewEnumerator9
      (Rendering|Components|Sprite|SetSprite (Variables|Default|GetPaperSprite) "/Game/Assets/Cards/whirlpool_card_Sprite.whirlpool_card_Sprite")
      (Variables|Default|SetAttack 40)
      (Variables|Default|SetDefense 0)
      (Variables|Default|SetStatusEffect "NewEnumerator5")
      (Variables|Default|SetStatusValue 50)
      (Variables|Default|SetEnergyCost 3))))