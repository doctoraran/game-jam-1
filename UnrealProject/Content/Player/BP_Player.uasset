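; BP_Player is a player combatant in a turn-based card game, holding health, opponents and a hand of cards.
; It registers with the GameState on BeginPlay, stores opponents passed at turn start minus itself, and sends attack input as a message targeting the first opponent.
; Damage lowers health and prints it, while SendCard spawns cards into the hand.
; Tick creates and adds new health and energy bar widgets every frame.
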(event Input|EnhancedActionEvents|EnhancedInputActionIA_Attack
  (params (ActionValue :type Boolean) (ElapsedSeconds :type Float%20%28double-precision%29) (TriggeredSeconds :type Float%20%28double-precision%29) (InputAction :type Input%20Action%20Object%20Reference :default "/Game/Player/IA_Attack.IA_Attack"))
  (:Started
    (Class|BPIAttack|Attack(Message) (Game|GetGameState) 2 self (Utilities|Array|Get(acopy) (Variables|Default|GetOpponents)))))

(event EventBeginPlay
  (Class|BPIRegisterTurn|RegisterTurn(Message) (Game|GetGameState) self))

(event EventSendCard
  (params (Card :type E_CardType%20Enum :default "NewEnumerator0"))
  (bind _returnvalue (Game|SpawnActorfromClass "/Game/BP_Card.BP_Card_C" (Transformation|GetActorTransform) "Undefined" "MultiplyWithRoot" 0 0))
  (Utilities|Array|Add (Variables|Default|GetHand) _returnvalue))

(event EventTick
  (params (DeltaSeconds :type Float%20%28single-precision%29))
  (bind _returnvalue (UserInterface|CreateWidget "/Game/UI/HealthAndEnergy/HealthBar.HealthBar_C"))
  (bind _returnvalue_2 (UserInterface|CreateWidget "/Game/UI/HealthAndEnergy/EnergyBar.EnergyBar_C"))
  (UserInterface|Viewport|AddtoViewport _returnvalue 0))

(event EventDoDamage
  (params (Damage :type Integer))
  (bind _output_get (Variables|Default|SetHealth (- (Variables|Default|GetHealth) Damage)))
  (Development|PrintString (Utilities|String|Append "Your Health is:" (Utilities|String|ToString(Integer) _output_get))))

(event EventStartTurn
  (params (Opponents :type Array%20of%20Actor%20Object%20References))
  (bind _output_get (Variables|Default|SetOpponents Opponents))
  (Utilities|Array|RemoveItem _output_get self))

(fn ConstructionScript
  (Variables|Default|SetHealth (Variables|Default|GetMaxHealth)))